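; Tamed Froggyman creature that wears corrupt armour with a frog mask, spear and shield, and hides its rider while mounted.
; BeginPlay assembles the outfit with master-pose meshes and body masks, then the server scales stats by AlphaTribe INI multipliers, reconciling some with saved values.
; CraftMultiplier scales SpeedMultiplier rather than a crafting stat.
; Damage triggers one-shot voice lines at health thresholds; death spawns a delayed explosion and sound.
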(event EventOnSetDeath
  ;[1 1 1] On death effects
  (Utilities|FlowControl|Delay 1.0)
  (bind _returnvalue (Effects|SpawnEmitteratLocation "/Game/PrimalEarth/Effects/Particles/Fire/PS_C4AirExplosionFire_OLD.PS_C4AirExplosionFire_OLD" (Transformation|GetActorLocation)))
  (Transformation|SetRelativeScale3D _returnvalue "5.000000,5.000000,5.000000")
  (Utilities|FlowControl|Delay 1.0)
  (Class|GameplayStatics|PlaySoundAttached (Variables|Default|GetDeath%20CUE) (Variables|Character|GetMesh))
  (Components|Activation|Deactivate (Variables|Default|GetSpearPS)))

(event EventBeginPlay
  (bind _pants (Variables|Default|GetPants))
  (bind _mesh (Variables|Character|GetMesh))
  (bind _shirt (Variables|Default|GetShirt))
  (bind _gloves (Variables|Default|GetGloves))
  (bind _boots (Variables|Default|GetBoots))
  (bind _bodymaskindex (Variables|Default|GetBodyMaskIndex))
  (bind _mesh_2 (Variables|Character|GetMesh))
  (bind _bodymaskindex_2 (Variables|Default|GetBodyMaskIndex))
  (bind _mesh_3 (Variables|Character|GetMesh))
  (bind _bodymaskindex_3 (Variables|Default|GetBodyMaskIndex))
  (bind _mesh_4 (Variables|Character|GetMesh))
  (bind _mesh_5 (Variables|Character|GetMesh))
  (bind _bodymaskindex_4 (Variables|Default|GetBodyMaskIndex))
  (bind _savegametorp (Variables|Default|GetSaveGameTorp))
  (bind _savegamefood (Variables|Default|GetSaveGameFood))
  (bind _savegamestam (Variables|Default|GetSaveGameStam))
  (bind _savegamehealth (Variables|Default|GetSaveGameHealth))
  (Utilities|FlowControl|Sequence
    (:then_0
      ;[1 1 1] Set equipment
      (Class|SkinnedMeshComponent|SetMasterPoseComponent _pants _mesh)
      (Class|SkinnedMeshComponent|SetSkeletalMesh _pants "/Game/PrimalEarth/Human/Male/Outfits/CorruptArmour/Pants/SK_Corrupt_Pants_RIG.SK_Corrupt_Pants_RIG")
      (bind _returnvalue (Rendering|Material|CreateDynamicMaterialInstance _mesh_2 _bodymaskindex (Rendering|Material|GetMaterial _mesh_2 _bodymaskindex) :!class /Script/Engine.PrimitiveComponent))
      (Rendering|Material|SetTextureParameterValue _returnvalue "BodyMask_Pants" (Variables|Default|GetPantsMask))
      (Class|SkinnedMeshComponent|SetMasterPoseComponent _shirt _mesh)
      (Class|SkinnedMeshComponent|SetSkeletalMesh _shirt "/Game/PrimalEarth/Human/Male/Outfits/CorruptArmour/Shirt/SK_HM_Corrupt_Shirt.SK_HM_Corrupt_Shirt")
      (bind _returnvalue_2 (Rendering|Material|CreateDynamicMaterialInstance _mesh_3 _bodymaskindex_2 (Rendering|Material|GetMaterial _mesh_3 _bodymaskindex_2) :!class /Script/Engine.PrimitiveComponent))
      (Rendering|Material|SetTextureParameterValue _returnvalue_2 "BodyMask_Shirt" (Variables|Default|GetShirtMask))
      (Class|SkinnedMeshComponent|SetMasterPoseComponent _gloves _mesh)
      (Class|SkinnedMeshComponent|SetSkeletalMesh _gloves "/Game/PrimalEarth/Human/Male/Outfits/CorruptArmour/Gloves/SK_HM_CorruptGloves.SK_HM_CorruptGloves")
      (bind _returnvalue_3 (Rendering|Material|CreateDynamicMaterialInstance _mesh_4 _bodymaskindex_3 (Rendering|Material|GetMaterial _mesh_4 _bodymaskindex_3) :!class /Script/Engine.PrimitiveComponent))
      (Rendering|Material|SetTextureParameterValue _returnvalue_3 "BodyMask_Gloves" (Variables|Default|GetGlovesMask))
      (Class|SkinnedMeshComponent|SetMasterPoseComponent _boots _mesh)
      (Class|SkinnedMeshComponent|SetSkeletalMesh _boots "/Game/PrimalEarth/Human/Male/Outfits/CorruptArmour/Boots/SK_CorruptedBoots_Male.SK_CorruptedBoots_Male")
      (bind _returnvalue_4 (Rendering|Material|CreateDynamicMaterialInstance _mesh_5 _bodymaskindex_4 (Rendering|Material|GetMaterial _mesh_5 _bodymaskindex_4) :!class /Script/Engine.PrimitiveComponent))
      (Rendering|Material|SetTextureParameterValue _returnvalue_4 "BodyMask_Boots" (Variables|Default|GetBootsMask))
      (Components|StaticMesh|SetStaticMesh (Variables|Default|GetHat) "/Game/Mods/AT/Core/SM/FroggyMask_SM.FroggyMask_SM")
      (Components|StaticMesh|SetStaticMesh (Variables|Default|GetLeftHand) "/Game/Mods/AT/Core/SM/FroggyShield_SM.FroggyShield_SM")
      (Components|StaticMesh|SetStaticMesh (Variables|Default|GetRightHand) "/Game/Mods/AT/Core/SM/FroggySpear_SM.FroggySpear_SM")
      (Components|StaticMesh|SetStaticMesh (Variables|Default|GetImplant) "/Game/PrimalEarth/Human/Male/Implants/SM_Implant_Alpha_Male_TPV.SM_Implant_Alpha_Male_TPV"))
    (:then_1
      ;[1 1 1] Sound CUE on spawn
      (Class|GameplayStatics|PlaySoundAttached (Variables|Default|GetSpawn%20CUE) (Variables|Character|GetMesh)))
    (:then_2
      ;[1 1 1] Lethals improved statmod
      (Utilities|FlowControl|Delay 0.2)
      (if (Networking|IsServer)
        (bind _asshootergamemode (Utilities|Casting|CastToShooterGameMode (Game|GetGameMode)))
        (bind _returnvalue_5 (Class|PrimalCharacter|GetCharacterStatusComponent))
        (Utilities|FlowControl|Sequence
          (:then_0
            (bind _returnvalue_6 (Class|ShooterGameMode|GetFloatOptionIni _asshootergamemode "AlphaTribe" "HealthMultiplier"))
            (Class|PrimalCharacterStatusComponent|SetMaxStatusValue _returnvalue_5 "Health" (* (Math|Float|SelectFloat _returnvalue_6 1.0 (> _returnvalue_6 0.0)) (Class|PrimalCharacterStatusComponent|BPGetMaxStatusValue _returnvalue_5 "Health")))
            (Class|PrimalCharacterStatusComponent|BPDirectSetCurrentStatusValue _returnvalue_5 "Health" (Math|Float|Min(Float) (Class|PrimalCharacterStatusComponent|BPGetMaxStatusValue _returnvalue_5 "Health") (Math|Float|SelectFloat (Math|Float|Max(Float) (Class|PrimalCharacterStatusComponent|BPGetCurrentStatusValue _returnvalue_5 "Health") _savegamehealth) (Class|PrimalCharacterStatusComponent|BPGetMaxStatusValue _returnvalue_5 "Health") (> _savegamehealth 0.0))))
            (Class|PrimalCharacterStatusComponent|UpdatedCurrentStatusValue _returnvalue_5 "Health" (Class|PrimalCharacterStatusComponent|BPGetCurrentStatusValue _returnvalue_5 "Health") true 0 true true))
          (:then_1
            (bind _returnvalue_7 (Class|ShooterGameMode|GetFloatOptionIni _asshootergamemode "AlphaTribe" "StamMultiplier"))
            (Class|PrimalCharacterStatusComponent|SetMaxStatusValue _returnvalue_5 "Stamina" (* (Math|Float|SelectFloat _returnvalue_7 1.0 (> _returnvalue_7 0.0)) (Class|PrimalCharacterStatusComponent|BPGetMaxStatusValue _returnvalue_5 "Stamina")))
            (Class|PrimalCharacterStatusComponent|BPDirectSetCurrentStatusValue _returnvalue_5 "Stamina" (Math|Float|Min(Float) (Class|PrimalCharacterStatusComponent|BPGetMaxStatusValue _returnvalue_5 "Stamina") (Math|Float|SelectFloat (Math|Float|Max(Float) (Class|PrimalCharacterStatusComponent|BPGetCurrentStatusValue _returnvalue_5 "Stamina") _savegamestam) (Class|PrimalCharacterStatusComponent|BPGetMaxStatusValue _returnvalue_5 "Stamina") (> _savegamestam 0.0))))
            (Class|PrimalCharacterStatusComponent|UpdatedCurrentStatusValue _returnvalue_5 "Stamina" (Class|PrimalCharacterStatusComponent|BPGetCurrentStatusValue _returnvalue_5 "Stamina") true 0 true true))
          (:then_2
            (bind _returnvalue_8 (Class|ShooterGameMode|GetFloatOptionIni _asshootergamemode "AlphaTribe" "WeightMultiplier"))
            (Class|PrimalCharacterStatusComponent|SetMaxStatusValue _returnvalue_5 "Weight" (* (Math|Float|SelectFloat _returnvalue_8 1.0 (> _returnvalue_8 0.0)) (Class|PrimalCharacterStatusComponent|BPGetMaxStatusValue _returnvalue_5 "Weight"))))
          (:then_3
            (bind _returnvalue_9 (Class|ShooterGameMode|GetFloatOptionIni _asshootergamemode "AlphaTribe" "DamageMultiplier"))
            (Class|PrimalCharacterStatusComponent|SetMaxStatusValue _returnvalue_5 "MeleeDamageMultiplier" (* (Math|Float|SelectFloat _returnvalue_9 1.0 (> _returnvalue_9 0.0)) (Class|PrimalCharacterStatusComponent|BPGetMaxStatusValue _returnvalue_5 "MeleeDamageMultiplier"))))
          (:then_4
            (bind _returnvalue_10 (Class|ShooterGameMode|GetFloatOptionIni _asshootergamemode "AlphaTribe" "SpeedMultiplier"))
            (Class|PrimalCharacterStatusComponent|SetMaxStatusValue _returnvalue_5 "SpeedMultiplier" (* (Math|Float|SelectFloat _returnvalue_10 1.0 (> _returnvalue_10 0.0)) (Class|PrimalCharacterStatusComponent|BPGetMaxStatusValue _returnvalue_5 "SpeedMultiplier"))))
          (:then_5
            (bind _returnvalue_11 (Class|ShooterGameMode|GetFloatOptionIni _asshootergamemode "AlphaTribe" "CraftMultiplier"))
            (Class|PrimalCharacterStatusComponent|SetMaxStatusValue _returnvalue_5 "SpeedMultiplier" (* (Math|Float|SelectFloat _returnvalue_11 1.0 (> _returnvalue_11 0.0)) (Class|PrimalCharacterStatusComponent|BPGetMaxStatusValue _returnvalue_5 "SpeedMultiplier"))))
          (:then_6
            (bind _returnvalue_12 (Class|ShooterGameMode|GetFloatOptionIni _asshootergamemode "AlphaTribe" "FoodMultiplier"))
            (Class|PrimalCharacterStatusComponent|SetMaxStatusValue _returnvalue_5 "Food" (* (Math|Float|SelectFloat _returnvalue_12 1.0 (> _returnvalue_12 0.0)) (Class|PrimalCharacterStatusComponent|BPGetMaxStatusValue _returnvalue_5 "Food")))
            (Class|PrimalCharacterStatusComponent|BPDirectSetCurrentStatusValue _returnvalue_5 "Food" (Math|Float|Min(Float) (Class|PrimalCharacterStatusComponent|BPGetMaxStatusValue _returnvalue_5 "Food") (Math|Float|SelectFloat (Math|Float|Max(Float) (Class|PrimalCharacterStatusComponent|BPGetCurrentStatusValue _returnvalue_5 "Food") _savegamefood) (Class|PrimalCharacterStatusComponent|BPGetMaxStatusValue _returnvalue_5 "Food") (> _savegamefood 0.0))))
            (Class|PrimalCharacterStatusComponent|UpdatedCurrentStatusValue _returnvalue_5 "Food" (Class|PrimalCharacterStatusComponent|BPGetCurrentStatusValue _returnvalue_5 "Food") true 0 true true))
          (:then_7
            (bind _returnvalue_13 (Class|ShooterGameMode|GetFloatOptionIni _asshootergamemode "AlphaTribe" "TorporMultiplier"))
            (Class|PrimalCharacterStatusComponent|SetMaxStatusValue _returnvalue_5 "Torpidity" (* (Math|Float|SelectFloat _returnvalue_13 1.0 (> _returnvalue_13 0.0)) (Class|PrimalCharacterStatusComponent|BPGetMaxStatusValue _returnvalue_5 "Torpidity")))
            (Class|PrimalCharacterStatusComponent|BPDirectSetCurrentStatusValue _returnvalue_5 "Torpidity" (Math|Float|Min(Float) (Class|PrimalCharacterStatusComponent|BPGetMaxStatusValue _returnvalue_5 "Torpidity") (Math|Float|SelectFloat (Math|Float|Min(Float) (Class|PrimalCharacterStatusComponent|BPGetCurrentStatusValue _returnvalue_5 "Torpidity") _savegametorp) (Class|PrimalCharacterStatusComponent|BPGetMaxStatusValue _returnvalue_5 "Torpidity") (> _savegametorp 0.0)) (Class|PrimalCharacterStatusComponent|BPGetCurrentStatusValue _returnvalue_5 "Torpidity")))
            (Class|PrimalCharacterStatusComponent|UpdatedCurrentStatusValue _returnvalue_5 "Torpidity" (Class|PrimalCharacterStatusComponent|BPGetCurrentStatusValue _returnvalue_5 "Torpidity") true 0 true true))
          (:then_8
            (Variables|Default|SetNotSaveGameStatModified true)))))))

(event EventPointDamage
  (params (Damage :type Float%20%28single-precision%29) (DamageType :type Damage%20Type%20Object%20Reference) (HitLocation :type Vector :default "0, 0, 0") (HitNormal :type Vector :default "0, 0, 0") (HitComponent :type Primitive%20Component%20Object%20Reference) (BoneName :type Name :default "None") (ShotFromDirection :type Vector :default "0, 0, 0") (InstigatedBy :type Controller%20Object%20Reference) (DamageCauser :type Actor%20Object%20Reference))
  (bind _mycharacterstatuscomponent (Variables|Default|GetMyCharacterStatusComponent))
  (bind _mesh (Variables|Character|GetMesh))
  (bind _returnvalue (Class|PrimalCharacterStatusComponent|BPGetPercentStatusValue _mycharacterstatuscomponent "Health"))
  ;[1 1 1] Sound at different health
  (if (Variables|Default|GetVoice75)
    (if (Variables|Default|GetVoice50) :!label _label
      (if (not (Variables|Default|GetVoice25)) :!label _label_2
        (if (<= _returnvalue 0.25)
          (Class|GameplayStatics|PlaySoundAttached (Variables|Default|GetSelectVoice25) _mesh)
          (Variables|Default|SetVoice25 true)))
      (elif (<= _returnvalue 0.5)
        (Class|GameplayStatics|PlaySoundAttached (Variables|Default|GetSelectVoice50) _mesh)
        (Variables|Default|SetVoice50 true)
        (else
          (goto _label_2))))
    (elif (<= _returnvalue 0.75)
      (Class|GameplayStatics|PlaySoundAttached (Variables|Default|GetSelectVoice75) _mesh)
      (Variables|Default|SetVoice75 true)
      (else
        (goto _label)))))

(fn ConstructionScript
  (|CallParentFunction))

(fn BPNotifySetRider
  (params (RiderSetting :type Shooter%20Character%20Object%20Reference))
  (Rendering|SetActorHiddenInGame RiderSetting true))

(fn BPNotifyClearRider
  (params (RiderClearing :type Shooter%20Character%20Object%20Reference))
  (Rendering|SetActorHiddenInGame RiderClearing false))